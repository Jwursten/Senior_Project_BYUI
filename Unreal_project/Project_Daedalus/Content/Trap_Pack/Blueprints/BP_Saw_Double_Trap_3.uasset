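; BP_Saw_Double_Trap_3 is a double saw trap that calls Death on a BP_FirstPersonCharacter that overlaps it.
; If TrapActivate is set on BeginPlay, two timelines, with play rates scaled by inverse SpeedRate, slide two saw holders along local X.
; The first timeline's updates also call RoleTick, which pitches two meshes by a RoleSpeed-based amount and re-runs itself through a half-second Delay loop.
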(event `Role Tick`
  ;[1 1 1] Role Events
  (`self.Role Rotation` (`self.Role Speed`) :!label _label)
  (`KismetSystemLibrary.Delay` 0.5)
  (goto _label))

(event `Role Rotation`
  (params (Speed :type "Float (double-precision)"))
  ;[1 1 1] Role Events
  (`SceneComponent.K2_AddLocalRotation` (`self.Mesh_4`) (`KismetMathLibrary.MakeRotator` 0.0 (* Speed (`self.Role Speed`))) false false)
  (`SceneComponent.K2_AddLocalRotation` (`self.Mesh_5`) (`KismetMathLibrary.MakeRotator` 0.0 (* Speed (`self.Role Speed`))) false false))

(event `self.ReceiveBeginPlay`
  (if (`self.Trap_Activate`)
    (`TimelineComponent.SetPlayRate` (`self. Timeline`) (/ 1.0 (`self.SpeedRate`)))
    (`TimelineComponent.SetPlayRate` (`self.Timeline_0`) (/ 1.0 (`self.SpeedRate`)))
    (`|ExecutionSequence`
      (:`then_0`
        (bind (_direction _newtrack_0) (`Timeline|Timeline`)
          (:`Update`
            (`SceneComponent.K2_SetRelativeLocation` (`self.Trap_2_Saw_Holder`) (`KismetMathLibrary.MakeVector` _newtrack_0 10.176977) false false)
            (`self.Role Tick`))))
      (:`then_1`
        (bind (_direction_2 _newtrack_0_2) (`Timeline|Timeline_0`)
          (:`Update`
            (`SceneComponent.K2_SetRelativeLocation` (`self.Trap_2_Saw_Holder1`) (`KismetMathLibrary.MakeVector` _newtrack_0_2 10.176977) false false)))))))

(event `self.ReceiveActorBeginOverlap`
  (params (OtherActor :type "Actor Object Reference"))
  (bind _asbp_first_person_character (cast `/Game/FirstPerson/Blueprints/BP_FirstPersonCharacter` OtherActor))
  (`/Game/FirstPerson/Blueprints/BP_FirstPersonCharacter.Death` _asbp_first_person_character))

(fn `UserConstructionScript`)