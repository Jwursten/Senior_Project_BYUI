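; BP_Spear_Trap is a trap actor that continuously fires spears from randomly chosen launch points.
; From BeginPlay, an endless Delay-based loop spawns a BP_Spear_Shot every half second, with no trigger or stop condition.
; Each spawn picks one of nine Arrow component world transforms at random and always spawns regardless of collision.
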(event `self.ReceiveBeginPlay`
  (bind _output (`|GetArrayItem` (`|MakeArray` (`SceneComponent.K2_GetComponentToWorld` (`self.Arrow`)) (`SceneComponent.K2_GetComponentToWorld` (`self.Arrow3`)) (`SceneComponent.K2_GetComponentToWorld` (`self.Arrow2`)) (`SceneComponent.K2_GetComponentToWorld` (`self.Arrow4`)) (`SceneComponent.K2_GetComponentToWorld` (`self.Arrow8`)) (`SceneComponent.K2_GetComponentToWorld` (`self.Arrow7`)) (`SceneComponent.K2_GetComponentToWorld` (`self.Arrow6`)) (`SceneComponent.K2_GetComponentToWorld` (`self.Arrow5`)) (`SceneComponent.K2_GetComponentToWorld` (`self.Arrow1`))) (`KismetMathLibrary.RandomInteger` 9)))
  (`|SpawnActorFromClass` "/Game/Trap_Pack/Blueprints/BP_Spear_Shot.BP_Spear_Shot_C" _output "AlwaysSpawn" "OverrideRootScale" null null :!label _label)
  (`KismetSystemLibrary.Delay` 0.5)
  (`|SpawnActorFromClass` "/Game/Trap_Pack/Blueprints/BP_Spear_Shot.BP_Spear_Shot_C" _output "AlwaysSpawn" "OverrideRootScale" null null)
  (`KismetSystemLibrary.Delay` 0.5)
  (goto _label))

(fn `UserConstructionScript`)