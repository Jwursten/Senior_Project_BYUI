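; BP_Trap_6 is a trap actor that kills the first-person player character on overlap.
; When TrapActivate is set, BeginPlay plays a timeline whose track drives the pitch of Mesh1, animating the trap's rotation.
; SpeedRate sets the timeline play rate as its reciprocal, so higher values slow the motion.
; Any overlapping BP_FirstPersonCharacter has Death called on it, regardless of whether the trap is activated.
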(event `self.ReceiveBeginPlay`
  (if (`self.Trap_Activate`)
    (`TimelineComponent.SetPlayRate` (`self. Timeline`) (/ 1.0 (`self.SpeedRate`)))
    (bind (_direction _newtrack_0) (`Timeline|Timeline`)
      (:`Update`
        (`SceneComponent.K2_SetRelativeRotation` (`self.Mesh_1`) (`KismetMathLibrary.MakeRotator` 0.0 _newtrack_0) false false)))))

(event `self.ReceiveActorBeginOverlap`
  (params (OtherActor :type "Actor Object Reference"))
  (bind _asbp_first_person_character (cast `/Game/FirstPerson/Blueprints/BP_FirstPersonCharacter` OtherActor))
  (`/Game/FirstPerson/Blueprints/BP_FirstPersonCharacter.Death` _asbp_first_person_character))

(fn `UserConstructionScript`)