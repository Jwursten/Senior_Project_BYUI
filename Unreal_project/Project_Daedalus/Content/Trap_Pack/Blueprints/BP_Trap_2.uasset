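; BP_Trap_2 is a trap that moves Mesh1 vertically and rolls it when TrapActivate is set at BeginPlay.
; A Timeline, with play rate set to the inverse of SpeedRate, drives the mesh's relative Z and calls RoleTick on every update.
; RoleTick adds local roll by RoleSpeed squared, then re-runs itself through a half-second Delay loop that continues independently of the Timeline.
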(event `Role Tick`
  ;[1 1 1] Role Events
  (`self.Role Rotation` (`self.Role Speed`) :!label _label)
  (`KismetSystemLibrary.Delay` 0.5)
  (goto _label))

(event `Role Rotation`
  (params (Speed :type "Float (double-precision)"))
  ;[1 1 1] Role Events
  (`SceneComponent.K2_AddLocalRotation` (`self.Mesh_1`) (`KismetMathLibrary.MakeRotator` (* Speed (`self.Role Speed`))) false false))

(event `self.ReceiveBeginPlay`
  (if (`self.Trap_Activate`)
    (`TimelineComponent.SetPlayRate` (`self. Timeline`) (/ 1.0 (`self.SpeedRate`)))
    (bind (_direction _newtrack_0) (`Timeline|Timeline`)
      (:`Update`
        (`SceneComponent.K2_SetRelativeLocation` (`self.Mesh_1`) (`KismetMathLibrary.MakeVector` 0.0 0.0 _newtrack_0) false false)
        (`self.Role Tick`)))))

(fn `UserConstructionScript`)