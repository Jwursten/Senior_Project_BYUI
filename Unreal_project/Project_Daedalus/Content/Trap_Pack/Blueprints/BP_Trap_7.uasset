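; BP_Trap_7 is a rotating trap actor that kills the first-person player character on overlap.
; On BeginPlay, if TrapActivate is set, two timelines drive the pitch of Mesh1 and Mesh3 separately, with play rate set to the inverse of SpeedRate.
; Any actor overlap that casts to BP_FirstPersonCharacter calls its Death function, regardless of TrapActivate.
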(event `self.ReceiveBeginPlay`
  (if (`self.Trap_Activate`)
    (`TimelineComponent.SetPlayRate` (`self. Timeline`) (/ 1.0 (`self.SpeedRate`)))
    (`TimelineComponent.SetPlayRate` (`self.Timeline_2`) (/ 1.0 (`self.SpeedRate`)))
    (`|ExecutionSequence`
      (:`then_0`
        (bind (_direction _newtrack_2) (`Timeline|Timeline`)
          (:`Update`
            (`SceneComponent.K2_SetRelativeRotation` (`self.Mesh_1`) (`KismetMathLibrary.MakeRotator` 0.0 _newtrack_2) false false))))
      (:`then_1`
        (bind (_direction_2 _newtrack_2_2) (`Timeline|Timeline_2`)
          (:`Update`
            (`SceneComponent.K2_SetRelativeRotation` (`self.Mesh_3`) (`KismetMathLibrary.MakeRotator` 0.0 _newtrack_2_2) false false)))))))

(event `self.ReceiveActorBeginOverlap`
  (params (OtherActor :type "Actor Object Reference"))
  (bind _asbp_first_person_character (cast `/Game/FirstPerson/Blueprints/BP_FirstPersonCharacter` OtherActor))
  (`/Game/FirstPerson/Blueprints/BP_FirstPersonCharacter.Death` _asbp_first_person_character))

(fn `UserConstructionScript`)