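; BP_Standing_Saw_Trap is a saw trap that kills the first-person character on overlap by calling Death.
; When TrapActivate is set, BeginPlay plays a Timeline at a rate randomized from MinSpeed and MaxSpeed, driving Mesh1's yaw.
; Each Timeline update also calls RoleTick, which adds yaw to Mesh3 scaled by RoleSpeed squared and loops through a Delay.
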(event `Role Tick`
  ;[1 1 1] Role Events
  (`self.Role Rotation` (`self.Role Speed`) :!label _label)
  (`KismetSystemLibrary.Delay` 0.5)
  (goto _label))

(event `Role Rotation`
  (params (Speed :type "Float (double-precision)"))
  ;[1 1 1] Role Events
  (`SceneComponent.K2_AddLocalRotation` (`self.Mesh_3`) (`KismetMathLibrary.MakeRotator` 0.0 0.0 (* Speed (`self.Role Speed`))) false false))

(event `self.ReceiveBeginPlay`
  (if (`self.Trap_Activate`)
    (`TimelineComponent.SetPlayRate` (`self. Timeline`) (/ 1.0 (`KismetMathLibrary.RandomFloatInRange` (`self.MinSpeed`) (`self.MaxSpeed`))))
    (bind (_direction _newtrack_0) (`Timeline|Timeline`)
      (:`Update`
        (`SceneComponent.K2_SetRelativeRotation` (`self.Mesh_1`) (`KismetMathLibrary.MakeRotator` 0.0 0.0 _newtrack_0) false false)
        (`self.Role Tick`)))))

(event `self.ReceiveActorBeginOverlap`
  (params (OtherActor :type "Actor Object Reference"))
  (bind _asbp_first_person_character (cast `/Game/FirstPerson/Blueprints/BP_FirstPersonCharacter` OtherActor))
  (`/Game/FirstPerson/Blueprints/BP_FirstPersonCharacter.Death` _asbp_first_person_character))

(fn `UserConstructionScript`)