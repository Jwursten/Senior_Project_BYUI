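; BP_Spike_Trap is a hazard actor that kills the first-person character when it overlaps the trap.
; On BeginPlay, if TrapActivate is set, a timeline plays at a randomized rate and drives the spikes' relative Z position.
; The timeline's Sfx event spawns an attached, attenuated metal sound, with pitch randomized separately from the same speed range.
; The overlap kill calls the character's Death function and does not check TrapActivate.
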(event `self.ReceiveBeginPlay`
  (bind _returnvalue (/ 1.0 (`KismetMathLibrary.RandomFloatInRange` (`self.MinSpeed`) (`self.MaxSpeed`))))
  (if (`self.Trap_Activate`)
    (`TimelineComponent.SetPlayRate` (`self.Spikes Timeline`) _returnvalue)
    (bind (_direction _newtrack_0) (`Timeline|Spikes Timeline`)
      (:`Update`
        _)
      (:`sfx`
        (`GameplayStatics.SpawnSoundAttached` "/Game/Free_Sounds_Pack/cue/Draw_Weapon_Metal_1-1_Cue.Draw_Weapon_Metal_1-1_Cue" (`self.Audio`) "None" (0.0 0.0 0.0) (struct) "KeepRelativeOffset" false 1.0 _returnvalue 0.0 "/Game/FirstPerson/Blueprints/Sounds/Attenuation/Attenuation_SpikeTrap.Attenuation_SpikeTrap" null)))
    (`SceneComponent.K2_SetRelativeLocation` (`self.Spikes`) (`KismetMathLibrary.MakeVector` 0.0 0.0 _newtrack_0) false false)))

(event `self.ReceiveActorBeginOverlap`
  (params (OtherActor :type "Actor Object Reference"))
  (bind _asbp_first_person_character (cast `/Game/FirstPerson/Blueprints/BP_FirstPersonCharacter` OtherActor))
  (`/Game/FirstPerson/Blueprints/BP_FirstPersonCharacter.Death` _asbp_first_person_character))

(fn `UserConstructionScript`)