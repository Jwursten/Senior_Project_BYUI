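; BP_Swinging_Log_Trap is a trap actor that swings a log and kills the first-person player character on contact.
; On BeginPlay, if TrapActivate is set, a Timeline drives Mesh1's relative roll.
; Its play rate is the inverse of a random value between MinSpeed and MaxSpeed, so that value acts as a duration scale.
; Any actor overlap that casts to BP_FirstPersonCharacter calls Death, independent of TrapActivate.
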(event `self.ReceiveBeginPlay`
  (if (`self.Trap_Activate`)
    (`TimelineComponent.SetPlayRate` (`self. Timeline`) (/ 1.0 (`KismetMathLibrary.RandomFloatInRange` (`self.MinSpeed`) (`self.MaxSpeed`))))
    (bind (_direction _newtrack_2) (`Timeline|Timeline`)
      (:`Update`
        (`SceneComponent.K2_SetRelativeRotation` (`self.Mesh_1`) (`KismetMathLibrary.MakeRotator` _newtrack_2) false false)))))

(event `self.ReceiveActorBeginOverlap`
  (params (OtherActor :type "Actor Object Reference"))
  (bind _asbp_first_person_character (cast `/Game/FirstPerson/Blueprints/BP_FirstPersonCharacter` OtherActor))
  (`/Game/FirstPerson/Blueprints/BP_FirstPersonCharacter.Death` _asbp_first_person_character))

(fn `UserConstructionScript`)